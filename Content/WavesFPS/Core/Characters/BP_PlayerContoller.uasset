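; Player controller for a wave-based FPS that owns the HUD and tracks score, health, wave number and coins.
; It creates WBP_HUD on BeginPlay, and Handle events update the stored values, then push them to the HUD.
; The death event checks the HUD health bar's percent rather than CurrentHealth; at zero it shows WBP_DeathScreen, enables the cursor and pauses the game.
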(event `self.ReceiveBeginPlay`
  (bind _returnvalue (`|CreateWidget` "/Game/WavesFPS/Core/UserInterface/WBP_HUD.WBP_HUD_C" self))
  (bind _output_get (set `self.MainHUD` _returnvalue))
  (`UserWidget.AddToViewport` _output_get 0))

(event `HandlePlayerDead`
  (`self.ShowDeathScreen`))

(event `HandleUpdateScore`
  (params (Value :type Integer))
  (`self.UpdateScore` Value))

(event `HandleUpdateHealthBar`
  (params (HitPoiints :type "Float (double-precision)"))
  (`self.UpdateHealth` HitPoiints))

(event `HandleUpdateWaveNumber`
  (`self.UpdateWaveNumber`))

(event `HandleUpdateCoinNumber`
  (`self.UpdateCoins`))

(fn `ShowDeathScreen`
  (if (<= (`ProgressBar.Percent` (`/Game/WavesFPS/Core/UserInterface/WBP_HUD.HealthBar` (`self.MainHUD`))) 0.0)
    (bind _returnvalue (`|CreateWidget` "/Game/WavesFPS/Core/UserInterface/WBP_DeathScreen.WBP_DeathScreen_C" self))
    (bind _output_get (set `self.DeathHUD` _returnvalue))
    (`UserWidget.AddToViewport` _output_get 0)
    (set `self.bShowMouseCursor` true)
    (`GameplayStatics.SetGamePaused` true)))

(fn `UpdateCoins`
  (bind _result (`/Engine/EditorBlueprintResources/StandardMacros.IncrementInt` (`self.CurrentCoinsNumber`))
    (:`  `
      (`/Game/WavesFPS/Core/UserInterface/WBP_HUD.UpdatedCoinsText` (`self.MainHUD`) _result))))

(fn `UpdateHealth`
  (params (HitPoints :type "Float (double-precision)"))
  (bind _output_get (set `self.CurrentHealth` (- (`self.CurrentHealth`) HitPoints)))
  (`/Game/WavesFPS/Core/UserInterface/WBP_HUD.UpdateHealthBar` (`self.MainHUD`) _output_get))

(fn `UpdateScore`
  (params (PointsToAdd :type Integer))
  (bind _output_get (set `self.PlayerScore` (+ PointsToAdd (`self.PlayerScore`))))
  (`/Game/WavesFPS/Core/UserInterface/WBP_HUD.UpdateScoreText` (`self.MainHUD`) _output_get))

(fn `UpdateWaveNumber`
  (bind _result (`/Engine/EditorBlueprintResources/StandardMacros.IncrementInt` (`self.CurrentWaveNumber`))
    (:`  `
      (`/Game/WavesFPS/Core/UserInterface/WBP_HUD.UpdateWaveText` (`self.MainHUD`) _result))))

(fn `UserConstructionScript`)