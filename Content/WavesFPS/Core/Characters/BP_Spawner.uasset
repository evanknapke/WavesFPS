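; BP_Spawner is the spawner actor in WavesFPS that places enemies and coins within its SpawnArea volume.
; SpawnEnemies and SpawnCoins each raise a running count before spawning that many actors, so every call yields a larger batch, with enemies growing faster than coins.
; Both use a shared SpawnActor function that randomizes X and Y inside the area's scaled extent and keeps Z at its center.
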(event `SpawnEnemies`
  ;[1 1 1] Spawns enemies and incremets the number of enemies spawned every round
  (bind _output_get (set `self.NumEnemies` (+ (`self.NumEnemies`) 2)))
  (for _ (range 1 (+ _output_get 1))
    (`self.SpawnActor` "/Game/WavesFPS/Core/Characters/BP_Enemy.BP_Enemy_C")))

(event `SpawnCoins`
  ;[1 1 1] Spawns coins and increments the number of coins spawned every round
  (bind _output_get (set `self.NumCoins` (+ (`self.NumCoins`) 1)))
  (for _ (range 1 (+ _output_get 1))
    (`self.SpawnActor` "/Game/WavesFPS/Core/Characters/BP_Coin.BP_Coin_C")))

(fn `SpawnActor`
  (params (ActorToBeSpawned :type "Actor Class Reference"))
  (bind _spawnarea (`self.SpawnArea`))
  (bind (_returnvalue_x _returnvalue_y _returnvalue_z) (`KismetMathLibrary.BreakVector` (`SceneComponent.K2_GetComponentLocation` _spawnarea)))
  (bind (_returnvalue_x_2 _returnvalue_y_2) (`KismetMathLibrary.BreakVector` (`KismetMathLibrary.RandomPointInBoundingBox` (`KismetMathLibrary.MakeVector` _returnvalue_x _returnvalue_y _returnvalue_z) (`BoxComponent.GetScaledBoxExtent` _spawnarea))))
  (`|SpawnActorFromClass` ActorToBeSpawned (`KismetMathLibrary.MakeTransform` (`KismetMathLibrary.MakeVector` _returnvalue_x_2 _returnvalue_y_2 _returnvalue_z)) "Undefined" "OverrideRootScale" null null))

(fn `UserConstructionScript`)